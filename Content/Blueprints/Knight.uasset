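; Knight chess piece Blueprint that supplies the knight's candidate moves on the board.
; GetAvailableMoves bounds-checks each of the eight L-shaped offsets from the current tile and collects those passing an empty-tile or different-team test.
; The board is a flat array indexed as X*8+Y, with the stride hardcoded.
; An event swaps the mesh's Body material, while SetChessPieceVariables is an empty stub.
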(event `/Game/Blueprints/BP_Interfaces/BI_Changeable_Material.SetMaterialOnActoors`
  (params (Mat :type "Material Object Reference"))
  (`PrimitiveComponent.SetMaterialByName` (`self.StaticMesh`) "Body" Mat))

(fn `GetAvailableMoves`
  (params (board :type "Array of /Game/Blueprints/ChessPiece Object Reference (by ref)") (tileCountX :type Integer) (tileCountY :type Integer))
  (returns (r :type "Array of Vector2D Structure"))
  (locals (rr :type "Array of Vector2D Structure") (x :type Integer) (y :type Integer))
  (bind _output (`|GetArrayItem` (`local.board`) (+ (* (`local.x`) 8) (`local.y`))))
  (bind _output_2 (`|GetArrayItem` (`local.board`) (+ (* (`local.x`) 8) (`local.y`))))
  (bind _output_3 (`|GetArrayItem` (`local.board`) (+ (* (`local.x`) 8) (`local.y`))))
  (bind _output_4 (`|GetArrayItem` (`local.board`) (+ (* (`local.x`) 8) (`local.y`))))
  (bind _output_5 (`|GetArrayItem` (`local.board`) (+ (* (`local.x`) 8) (`local.y`))))
  (bind _output_6 (`|GetArrayItem` (`local.board`) (+ (* (`local.x`) 8) (`local.y`))))
  (bind _output_7 (`|GetArrayItem` (`local.board`) (+ (* (`local.x`) 8) (`local.y`))))
  (bind _output_8 (`|GetArrayItem` (`local.board`) (+ (* (`local.x`) 8) (`local.y`))))
  (`|ExecutionSequence`
    (:`then_0`
      ;[0 0 0 1 40] Top Movement
      ;;[0 0 0] Top Bottom Right
      (set `local.x` (+ (`self.currentX`) 1))
      (set `local.y` (+ (`self.currentY`) 2))
      (if (and (< (`local.x`) (`local.tileCountX`)) (< (`local.y`) (`local.tileCountY`)))
        (if (or (and (== _output_2 "/Game/Blueprints/Nones.Nones") (`|EnumEquality` (`/Game/Blueprints/ChessPiece.type` _output_2) "NewEnumerator8")) (!= (`/Game/Blueprints/ChessPiece.team` _output_2) (`self.team`)))
          (`KismetArrayLibrary.Array_Add` (`local.rr`) (`KismetMathLibrary.MakeVector2D` (`KismetMathLibrary.Conv_IntToDouble` (`local.x`)) (`KismetMathLibrary.Conv_IntToDouble` (`local.y`)))))))
    (:`then_1`
      ;;[0 0 0] Top Top Right
      (set `local.x` (+ (`self.currentX`) 2))
      (set `local.y` (+ (`self.currentY`) 1))
      (if (and (< (`local.x`) (`local.tileCountX`)) (< (`local.y`) (`local.tileCountY`)))
        (if (or (and (== _output_5 "/Game/Blueprints/Nones.Nones") (`|EnumEquality` (`/Game/Blueprints/ChessPiece.type` _output_5) "NewEnumerator8")) (!= (`/Game/Blueprints/ChessPiece.team` _output_5) (`self.team`)))
          (`KismetArrayLibrary.Array_Add` (`local.rr`) (`KismetMathLibrary.MakeVector2D` (`KismetMathLibrary.Conv_IntToDouble` (`local.x`)) (`KismetMathLibrary.Conv_IntToDouble` (`local.y`)))))))
    (:`then_2`
      ;;[0 0 0] Top Top Left
      (set `local.x` (+ (`self.currentX`) -1))
      (set `local.y` (+ (`self.currentY`) 2))
      (if (and (>= (`local.x`) 0) (< (`local.y`) (`local.tileCountY`)))
        (if (or (and (== _output_4 "/Game/Blueprints/Nones.Nones") (`|EnumEquality` (`/Game/Blueprints/ChessPiece.type` _output_4) "NewEnumerator8")) (!= (`/Game/Blueprints/ChessPiece.team` _output_4) (`self.team`)))
          (`KismetArrayLibrary.Array_Add` (`local.rr`) (`KismetMathLibrary.MakeVector2D` (`KismetMathLibrary.Conv_IntToDouble` (`local.x`)) (`KismetMathLibrary.Conv_IntToDouble` (`local.y`)))))))
    (:`then_3`
      ;;[0 0 0] Top Bottom Left
      (set `local.x` (+ (`self.currentX`) -2))
      (set `local.y` (+ (`self.currentY`) 1))
      (if (and (>= (`local.x`) 0) (< (`local.y`) (`local.tileCountY`)))
        (if (or (and (== _output "/Game/Blueprints/Nones.Nones") (`|EnumEquality` (`/Game/Blueprints/ChessPiece.type` _output) "NewEnumerator8")) (!= (`/Game/Blueprints/ChessPiece.team` _output) (`self.team`)))
          (`KismetArrayLibrary.Array_Add` (`local.rr`) (`KismetMathLibrary.MakeVector2D` (`KismetMathLibrary.Conv_IntToDouble` (`local.x`)) (`KismetMathLibrary.Conv_IntToDouble` (`local.y`)))))))
    (:`then_4`
      ;[0 0 0 1 40] BottomMovement
      ;;[0 0 0] Bottom Bottom Right
      (set `local.x` (+ (`self.currentX`) 1))
      (set `local.y` (+ (`self.currentY`) -2))
      (if (and (< (`local.x`) (`local.tileCountX`)) (>= (`local.y`) 0))
        (if (or (and (== _output_6 "/Game/Blueprints/Nones.Nones") (`|EnumEquality` (`/Game/Blueprints/ChessPiece.type` _output_6) "NewEnumerator8")) (!= (`/Game/Blueprints/ChessPiece.team` _output_6) (`self.team`)))
          (`KismetArrayLibrary.Array_Add` (`local.rr`) (`KismetMathLibrary.MakeVector2D` (`KismetMathLibrary.Conv_IntToDouble` (`local.x`)) (`KismetMathLibrary.Conv_IntToDouble` (`local.y`)))))))
    (:`then_5`
      ;;[0 0 0] Bottom Top Right
      (set `local.x` (+ (`self.currentX`) 2))
      (set `local.y` (+ (`self.currentY`) -1))
      (if (and (< (`local.x`) (`local.tileCountX`)) (>= (`local.y`) 0))
        (if (or (and (== _output_7 "/Game/Blueprints/Nones.Nones") (`|EnumEquality` (`/Game/Blueprints/ChessPiece.type` _output_7) "NewEnumerator8")) (!= (`/Game/Blueprints/ChessPiece.team` _output_7) (`self.team`)))
          (`KismetArrayLibrary.Array_Add` (`local.rr`) (`KismetMathLibrary.MakeVector2D` (`KismetMathLibrary.Conv_IntToDouble` (`local.x`)) (`KismetMathLibrary.Conv_IntToDouble` (`local.y`)))))))
    (:`then_6`
      ;;[0 0 0] Bottom Top Left
      (set `local.x` (+ (`self.currentX`) -1))
      (set `local.y` (+ (`self.currentY`) -2))
      (if (and (>= (`local.x`) 0) (>= (`local.y`) 0))
        (if (or (and (== _output_8 "/Game/Blueprints/Nones.Nones") (`|EnumEquality` (`/Game/Blueprints/ChessPiece.type` _output_8) "NewEnumerator8")) (!= (`/Game/Blueprints/ChessPiece.team` _output_8) (`self.team`)))
          (`KismetArrayLibrary.Array_Add` (`local.rr`) (`KismetMathLibrary.MakeVector2D` (`KismetMathLibrary.Conv_IntToDouble` (`local.x`)) (`KismetMathLibrary.Conv_IntToDouble` (`local.y`)))))))
    (:`then_7`
      ;;[0 0 0] Bottom Bottom Left
      (set `local.x` (+ (`self.currentX`) -2))
      (set `local.y` (+ (`self.currentY`) -1))
      (if (and (>= (`local.x`) 0) (>= (`local.y`) 0))
        (if (or (and (== _output_3 "/Game/Blueprints/Nones.Nones") (`|EnumEquality` (`/Game/Blueprints/ChessPiece.type` _output_3) "NewEnumerator8")) (!= (`/Game/Blueprints/ChessPiece.team` _output_3) (`self.team`)))
          (`KismetArrayLibrary.Array_Add` (`local.rr`) (`KismetMathLibrary.MakeVector2D` (`KismetMathLibrary.Conv_IntToDouble` (`local.x`)) (`KismetMathLibrary.Conv_IntToDouble` (`local.y`)))))))
    (:`then_8`
      (return (`local.rr`)))))

(fn `SetChessPieceVariables`
  (params (type_enum :type "/Game/Blueprints/ChessPieceType Enum (by ref)" :default "NewEnumerator8") (team_int :type "Integer (by ref)") (cp_actor :type "Actor Object Reference (by ref)"))
  (returns (cpnew :type "/Game/Blueprints/ChessPiece Object Reference"))
  (return null))

(fn `UserConstructionScript`
  (`parent.UserConstructionScript`))