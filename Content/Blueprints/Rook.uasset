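; Rook chess piece Blueprint that computes its available moves and can swap its mesh's Body material.
; GetAvailableMoves scans the flattened board (stride 8) along four straight directions, collecting empty and enemy squares.
; A shared Br flag stops scanning at an enemy and is never reset between directions; friendly pieces do not stop the scan.
; SetChessPieceVariables is an empty stub.
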(event `/Game/Blueprints/BP_Interfaces/BI_Changeable_Material.SetMaterialOnActoors`
  (params (Mat :type "Material Object Reference"))
  (`PrimitiveComponent.SetMaterialByName` (`self.StaticMesh`) "Body" Mat))

(fn `GetAvailableMoves`
  (params (board :type "Array of /Game/Blueprints/ChessPiece Object Reference (by ref)") (tileCountX :type Integer) (tileCountY :type Integer))
  (returns (r :type "Array of Vector2D Structure"))
  (locals (rr :type "Array of Vector2D Structure") (direction :type Integer) (i :type Integer) (br :type Boolean :default true))
  (bind _output (`|GetArrayItem` (`local.board`) (+ (* (`local.i`) 8) (`self.currentY`))))
  (bind _output_2 (`|GetArrayItem` (`local.board`) (+ (* (`self.currentX`) 8) (`local.i`))))
  (bind _output_3 (`|GetArrayItem` (`local.board`) (+ (* (`self.currentX`) 8) (`local.i`))))
  (bind _output_4 (`|GetArrayItem` (`local.board`) (+ (* (`local.i`) 8) (`self.currentY`))))
  (if (!= (`self.team`) -1)
    (if (== (`self.team`) 0)
      (set `local.direction` 1)
      (else
        (set `local.direction` -1)))
    (`|ExecutionSequence`
      (:`then_0`
        ;[0.4864 1 0] Down
        (set `local.i` (- (`self.currentY`) 1))
        (while (and (>= (`local.i`) 0) (`local.br`)) :!label _label
          (`|ExecutionSequence`
            (:`then_0`
              (if (`|EnumEquality` (`/Game/Blueprints/ChessPiece.type` (`|GetArrayItem` (`local.board`) (+ (* (`self.currentX`) 8) (`local.i`)))) "NewEnumerator8")
                (`KismetArrayLibrary.Array_Add` (`local.rr`) (`KismetMathLibrary.MakeVector2D` (`KismetMathLibrary.Conv_IntToDouble` (`self.currentX`)) (`KismetMathLibrary.Conv_IntToDouble` (`local.i`))))))
            (:`then_1`
              (if (`|EnumInequality` (`/Game/Blueprints/ChessPiece.type` _output_2) "NewEnumerator8")
                (if (!= (`/Game/Blueprints/ChessPiece.team` _output_2) (`self.team`))
                  (`KismetArrayLibrary.Array_Add` (`local.rr`) (`KismetMathLibrary.MakeVector2D` (`KismetMathLibrary.Conv_IntToDouble` (`self.currentX`)) (`KismetMathLibrary.Conv_IntToDouble` (`local.i`))))
                  (set `local.br` false)
                  (goto _label))))
            (:`then_2`
              (bind _result (`/Engine/EditorBlueprintResources/StandardMacros.DecrementInt` (`local.i`))
                (:`  `
                  (set `local.i` _result)
                  (goto _label)))))))
      (:`then_1`
        ;[0.4841 0 1] Up
        (set `local.i` (+ (`self.currentY`) 1))
        (while (and (< (`local.i`) (`local.tileCountY`)) (`local.br`)) :!label _label_2
          (`|ExecutionSequence`
            (:`then_0`
              (if (`|EnumEquality` (`/Game/Blueprints/ChessPiece.type` (`|GetArrayItem` (`local.board`) (+ (* (`self.currentX`) 8) (`local.i`)))) "NewEnumerator8")
                (`KismetArrayLibrary.Array_Add` (`local.rr`) (`KismetMathLibrary.MakeVector2D` (`KismetMathLibrary.Conv_IntToDouble` (`self.currentX`)) (`KismetMathLibrary.Conv_IntToDouble` (`local.i`))))))
            (:`then_1`
              (if (`|EnumInequality` (`/Game/Blueprints/ChessPiece.type` _output_3) "NewEnumerator8")
                (if (!= (`/Game/Blueprints/ChessPiece.team` _output_3) (`self.team`))
                  (`KismetArrayLibrary.Array_Add` (`local.rr`) (`KismetMathLibrary.MakeVector2D` (`KismetMathLibrary.Conv_IntToDouble` (`self.currentX`)) (`KismetMathLibrary.Conv_IntToDouble` (`local.i`))))
                  (set `local.br` false)
                  (goto _label_2))))
            (:`then_2`
              (bind _result_2 (`/Engine/EditorBlueprintResources/StandardMacros.IncrementInt` (`local.i`))
                (:`  `
                  (set `local.i` _result_2)
                  (goto _label_2)))))))
      (:`then_2`
        ;[0 1 0.9864] Left
        (set `local.i` (- (`self.currentX`) 1))
        (while (and (>= (`local.i`) 0) (`local.br`)) :!label _label_3
          (`|ExecutionSequence`
            (:`then_0`
              (if (`|EnumEquality` (`/Game/Blueprints/ChessPiece.type` (`|GetArrayItem` (`local.board`) (+ (* (`local.i`) 8) (`self.currentY`)))) "NewEnumerator8")
                (`KismetArrayLibrary.Array_Add` (`local.rr`) (`KismetMathLibrary.MakeVector2D` (`KismetMathLibrary.Conv_IntToDouble` (`local.i`)) (`KismetMathLibrary.Conv_IntToDouble` (`self.currentY`))))))
            (:`then_1`
              (if (`|EnumInequality` (`/Game/Blueprints/ChessPiece.type` _output_4) "NewEnumerator8")
                (if (!= (`/Game/Blueprints/ChessPiece.team` _output_4) (`self.team`))
                  (`KismetArrayLibrary.Array_Add` (`local.rr`) (`KismetMathLibrary.MakeVector2D` (`KismetMathLibrary.Conv_IntToDouble` (`local.i`)) (`KismetMathLibrary.Conv_IntToDouble` (`self.currentY`))))
                  (set `local.br` false)
                  (goto _label_3))))
            (:`then_2`
              (bind _result_3 (`/Engine/EditorBlueprintResources/StandardMacros.DecrementInt` (`local.i`))
                (:`  `
                  (set `local.i` _result_3)
                  (goto _label_3)))))))
      (:`then_3`
        ;[1 0 0] Right
        (set `local.i` (+ (`self.currentX`) 1))
        (while (and (< (`local.i`) (`local.tileCountX`)) (`local.br`)) :!label _label_4
          (`|ExecutionSequence`
            (:`then_0`
              (if (`|EnumEquality` (`/Game/Blueprints/ChessPiece.type` (`|GetArrayItem` (`local.board`) (+ (* (`local.i`) 8) (`self.currentY`)))) "NewEnumerator8")
                (`KismetArrayLibrary.Array_Add` (`local.rr`) (`KismetMathLibrary.MakeVector2D` (`KismetMathLibrary.Conv_IntToDouble` (`local.i`)) (`KismetMathLibrary.Conv_IntToDouble` (`self.currentY`))))))
            (:`then_1`
              (if (`|EnumInequality` (`/Game/Blueprints/ChessPiece.type` _output) "NewEnumerator8")
                (if (!= (`/Game/Blueprints/ChessPiece.team` _output) (`self.team`))
                  (`KismetArrayLibrary.Array_Add` (`local.rr`) (`KismetMathLibrary.MakeVector2D` (`KismetMathLibrary.Conv_IntToDouble` (`local.i`)) (`KismetMathLibrary.Conv_IntToDouble` (`self.currentY`))))
                  (set `local.br` false)
                  (goto _label_4))))
            (:`then_2`
              (bind _result_4 (`/Engine/EditorBlueprintResources/StandardMacros.IncrementInt` (`local.i`))
                (:`  `
                  (set `local.i` _result_4)
                  (goto _label_4)))))))
      (:`then_4`
        ;[0.08228 0.1878 0.402] Return
        (return (`local.rr`))))))

(fn `SetChessPieceVariables`
  (params (type_enum :type "/Game/Blueprints/ChessPieceType Enum (by ref)" :default "NewEnumerator8") (team_int :type "Integer (by ref)") (cp_actor :type "Actor Object Reference (by ref)"))
  (returns (cpnew :type "/Game/Blueprints/ChessPiece Object Reference"))
  (return null))

(fn `UserConstructionScript`
  (`parent.UserConstructionScript`))