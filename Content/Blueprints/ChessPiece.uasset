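; Base-style chess piece actor that moves and resizes smoothly on the board and exposes move-query functions.
; SetPosition and SetScale store target values that Tick eases toward with a delta-time-scaled lerp, or snap immediately when Force is set.
; GetAvailableMoves and GetSpecialMoves are stubs that ignore their inputs, returning four hardcoded central tiles and a fixed enum value.
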(event `self.ReceiveTick`
  (params (DeltaSeconds :type "Float (single-precision)"))
  (bind _returnvalue (* DeltaSeconds 10.0))
  (`self.K2_SetActorLocation` (`KismetMathLibrary.VLerp` (`self.K2_GetActorLocation`) (`self.desiredPosition`) _returnvalue))
  (`self.SetActorScale3D` (`KismetMathLibrary.VLerp` (`self.GetActorScale3D`) (`self.desiredScale`) _returnvalue)))

(fn `GetAvailableMoves`
  (params (board :type "Array of /Game/Blueprints/ChessPiece Object Reference") (tileCountX :type Integer) (tileCountY :type Integer))
  (returns (r :type "Array of Vector2D Structure"))
  (locals (rrr :type "Array of Vector2D Structure"))
  (bind _rrr (`local.rrr`))
  (`KismetArrayLibrary.Array_Add` _rrr (3.0 3.0))
  (`KismetArrayLibrary.Array_Add` _rrr (3.0 4.0))
  (`KismetArrayLibrary.Array_Add` _rrr (4.0 3.0))
  (`KismetArrayLibrary.Array_Add` _rrr (4.0 4.0))
  (return _rrr))

(fn `GetSpecialMoves`
  (params (board :type "Array of /Game/Blueprints/ChessPiece Object Reference") (moveList :type "Array of /Game/Blueprints/Vector2IntArray Structure") (availableMoves :type "Array of Vector2D Structure"))
  (returns (sp :type "/Game/Blueprints/SpecialMove Enum"))
  (return "NewEnumerator0"))

(fn `SetPosition`
  (params (position :type "Vector Structure") (force :type Boolean))
  (bind _output_get (set `self.desiredPosition` position))
  (if force
    (`self.K2_SetActorLocation` _output_get)))

(fn `SetScale`
  (params (scale :type "Vector Structure") (force :type Boolean))
  (bind _output_get (set `self.desiredScale` scale))
  (if force
    (`self.SetActorScale3D` _output_get)))

(fn `UserConstructionScript`)