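; Chess pawn piece that works out its legal-move candidates and sets its body material.
; GetAvailableMoves indexes a flattened eight-wide board to collect forward steps, double steps from the starting row and diagonal captures, with direction set by team.
; GetSpecialMoves flags promotion one row before the last, or checks the move list for en passant, appending that capture and returning the special-move type.
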(event `/Game/Blueprints/BP_Interfaces/BI_Changeable_Material.SetMaterialOnActoors`
  (params (Mat :type "Material Object Reference"))
  (`PrimitiveComponent.SetMaterialByName` (`self.StaticMesh`) "Body" Mat))

(fn `GetAvailableMoves`
  (params (board :type "Array of /Game/Blueprints/ChessPiece Object Reference (by ref)") (tileCountX :type Integer) (tileCountY :type Integer))
  (returns (r :type "Array of Vector2D Structure"))
  (locals (rr :type "Array of Vector2D Structure") (direction :type Integer) (index :type Integer) (indX2 :type Integer))
  (bind _output (`|GetArrayItem` (`local.board`) (`local.indX2`)))
  (bind _output_2 (`|GetArrayItem` (`local.board`) (`local.indX2`)))
  (if (!= (`self.team`) -1)
    (if (== (`self.team`) 0)
      (set `local.direction` 1)
      (else
        (set `local.direction` -1)))
    (bind _output_get (set `local.index` (+ (* (`self.currentX`) 8) (+ (`self.currentY`) (`local.direction`)))))
    (`|ExecutionSequence`
      (:`then_0`
        (bind _returnvalue (`|EnumEquality` (`/Game/Blueprints/ChessPiece.type` (`|GetArrayItem` board _output_get)) "NewEnumerator8"))
        ;[0.3961 0.9608 1] For Moving 1 step forward
        (if _returnvalue
          (`KismetArrayLibrary.Array_Add` (`local.rr`) (`KismetMathLibrary.MakeVector2D` (`KismetMathLibrary.Conv_IntToDouble` (`self.currentX`)) (`KismetMathLibrary.Conv_IntToDouble` (+ (`self.currentY`) (`local.direction`)))))))
      (:`then_1`
        ;[0.3961 0.9608 1] For Moving 2 Step forward
        (if _returnvalue
          (set `local.indX2` (+ (* (`self.currentX`) 8) (`self.currentY`) (* (`local.direction`) 2)))
          (`|ExecutionSequence`
            (:`then_0`
              ;;[1 1 1] WhiteTeam
              (if (and (== (`self.team`) 0) (== (`self.currentY`) 1) (`|EnumEquality` (`/Game/Blueprints/ChessPiece.type` (`|GetArrayItem` (`local.board`) (`local.indX2`))) "NewEnumerator8"))
                (`KismetArrayLibrary.Array_Add` (`local.rr`) (`KismetMathLibrary.MakeVector2D` (`KismetMathLibrary.Conv_IntToDouble` (`self.currentX`)) (`KismetMathLibrary.Conv_IntToDouble` (+ (`self.currentY`) (* (`local.direction`) 2)))))))
            (:`then_1`
              ;;[0 0 0] WhiteTeam
              (if (and (== (`self.team`) 1) (== (`self.currentY`) 6) (`|EnumEquality` (`/Game/Blueprints/ChessPiece.type` (`|GetArrayItem` (`local.board`) (`local.indX2`))) "NewEnumerator8"))
                (`KismetArrayLibrary.Array_Add` (`local.rr`) (`KismetMathLibrary.MakeVector2D` (`KismetMathLibrary.Conv_IntToDouble` (`self.currentX`)) (`KismetMathLibrary.Conv_IntToDouble` (+ (`self.currentY`) (* (`local.direction`) 2))))))))))
      (:`then_2`
        ;[0.3961 0.9608 1] Kill Moves Right
        (if (!= (`self.currentX`) (- (`local.tileCountX`) 1))
          (set `local.indX2` (+ (* (+ (`self.currentX`) 1) 8) (+ (`self.currentY`) (`local.direction`))))
          (if (and (`|EnumInequality` (`/Game/Blueprints/ChessPiece.type` _output_2) "NewEnumerator8") (!= (`/Game/Blueprints/ChessPiece.team` _output_2) (`self.team`)))
            (`KismetArrayLibrary.Array_Add` (`local.rr`) (`KismetMathLibrary.MakeVector2D` (`KismetMathLibrary.Conv_IntToDouble` (+ (`self.currentX`) 1)) (`KismetMathLibrary.Conv_IntToDouble` (+ (`self.currentY`) (`local.direction`))))))))
      (:`then_3`
        ;[0.3961 0.9608 1] Kill Moves Left
        (if (!= (`self.currentX`) 0)
          (set `local.indX2` (+ (* (+ (`self.currentX`) -1) 8) (+ (`self.currentY`) (`local.direction`))))
          (if (and (`|EnumInequality` (`/Game/Blueprints/ChessPiece.type` _output) "NewEnumerator8") (!= (`/Game/Blueprints/ChessPiece.team` _output) (`self.team`)))
            (`KismetArrayLibrary.Array_Add` (`local.rr`) (`KismetMathLibrary.MakeVector2D` (`KismetMathLibrary.Conv_IntToDouble` (+ (`self.currentX`) -1)) (`KismetMathLibrary.Conv_IntToDouble` (+ (`self.currentY`) (`local.direction`))))))))
      (:`then_4`
        ;[0.159 0.01229 0.2307 1 30] Returns R
        (return (`local.rr`))))))

(fn `GetSpecialMoves`
  (params (board :type "Array of /Game/Blueprints/ChessPiece Object Reference (by ref)") (moveList :type "Array of /Game/Blueprints/Vector2IntArray Structure (by ref)") (availableMoves :type "Array of Vector2D Structure (by ref)"))
  (returns (sp :type "/Game/Blueprints/SpecialMove Enum"))
  (locals (direction :type Integer) (lastMove :type "Array of Vector2D Structure"))
  (bind _lastmove (`local.lastMove`))
  (bind _returnvalue (`KismetArrayLibrary.Array_Length` (`local.moveList`)))
  (bind (_output_x _output_y) (`KismetMathLibrary.BreakVector2D` (`|GetArrayItem` (`local.lastMove`) 1)))
  (bind _output_x_2 (`KismetMathLibrary.BreakVector2D` (`|GetArrayItem` (`local.lastMove`) 1)))
  (bind (_output_x_3 _output_y_2) (`KismetMathLibrary.BreakVector2D` (`|GetArrayItem` _lastmove)))
  (bind (_output_x_4 _output_y_3) (`KismetMathLibrary.BreakVector2D` (`|GetArrayItem` _lastmove 1)))
  (bind (_output_x_5 _output_y_4) (`KismetMathLibrary.BreakVector2D` (`|GetArrayItem` (`local.lastMove`) 1)))
  (bind (_output_x_6 _output_y_5) (`KismetMathLibrary.BreakVector2D` (`|GetArrayItem` (`local.lastMove`) 1)))
  (bind _output_x_7 (`KismetMathLibrary.BreakVector2D` (`|GetArrayItem` (`local.lastMove`) 1)))
  (bind _output_val (break `/Game/Blueprints/Vector2IntArray` (`|GetArrayItem` (`local.moveList`) (- _returnvalue 1))))
  (if (!= (`self.team`) -1)
    (if (== (`self.team`) 0)
      (set `local.direction` 1)
      (else
        (set `local.direction` -1)))
    (`|ExecutionSequence`
      (:`then_0`
        ;[1 0 0] Promotion(of sort)
        (if (or (and (== (`self.team`) 0) (== (`self.currentY`) 6)) (and (== (`self.team`) 1) (== (`self.currentY`) 1)))
          (return "NewEnumerator3")))
      (:`then_1`
        ;[1 0 0] En Passant
        (if (> _returnvalue 0)
          (set `local.lastMove` _output_val)
          ;;[1 1 1] If the last piece moved was pawn
          (if (`|EnumEquality` (`/Game/Blueprints/ChessPiece.type` (`|GetArrayItem` (`local.board`) (`KismetMathLibrary.FTrunc` (+ (* _output_x 8) _output_y)))) "NewEnumerator1")
            ;;;[1 1 1] If the last move was a + 2 in either diection
            (if (== (`KismetMathLibrary.Abs_Int` (`KismetMathLibrary.FTrunc` (- _output_y_2 _output_y_3))) 2)
              ;;;;[1 1 1] If the last move was from the other team
              (if (!= (`/Game/Blueprints/ChessPiece.team` (`|GetArrayItem` (`local.board`) (`KismetMathLibrary.FTrunc` (+ (* _output_x_5 8) _output_y_4)))) (`self.team`))
                ;;;;;[1 1 1] If both pawns are on same Y
                (if (== (`KismetMathLibrary.FTrunc` _output_y_5) (`self.currentY`))
                  (`|ExecutionSequence`
                    (:`then_0`
                      ;;;;;;[1 1 1] Landed Left
                      (if (== (`KismetMathLibrary.FTrunc` _output_x_2) (- (`self.currentX`) 1))
                        (`KismetArrayLibrary.Array_Add` (`local.availableMoves`) (`KismetMathLibrary.MakeVector2D` (`KismetMathLibrary.Conv_IntToDouble` (- (`self.currentX`) 1)) (`KismetMathLibrary.Conv_IntToDouble` (+ (`self.currentY`) (`local.direction`)))))
                        (return "NewEnumerator1")))
                    (:`then_1`
                      ;;;;;;[1 1 1] Landed Right
                      (if (== (`KismetMathLibrary.FTrunc` _output_x_7) (+ (`self.currentX`) 1))
                        (`KismetArrayLibrary.Array_Add` (`local.availableMoves`) (`KismetMathLibrary.MakeVector2D` (`KismetMathLibrary.Conv_IntToDouble` (+ (`self.currentX`) 1)) (`KismetMathLibrary.Conv_IntToDouble` (+ (`self.currentY`) (`local.direction`)))))
                        (return "NewEnumerator1"))))))))))
      (:`then_2`
        ;[0 0 0] FinalCase
        (return "NewEnumerator0")))))

(fn `SetChessPieceVariables`
  (params (type_enum :type "/Game/Blueprints/ChessPieceType Enum (by ref)" :default "NewEnumerator8") (team_int :type "Integer (by ref)") (cp_actor :type "Actor Object Reference (by ref)"))
  (returns (cpnew :type "/Game/Blueprints/ChessPiece Object Reference"))
  (return null))

(fn `UserConstructionScript`
  (`parent.UserConstructionScript`))